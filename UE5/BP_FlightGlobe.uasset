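; Globe actor that plots flight routes from the Rotalar data table as debug-drawn splines, with a pin at Istanbul.
; LatLonToVector converts latitude/longitude to local positions, setting routes slightly below the pin's radius.
; Each row with Sira 0 starts a new spline; every row appends a point to the current one.
; Construction Script and BeginPlay duplicate this build; BeginPlay also colours splines and runs "show Splines".
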(event EventBeginPlay
  (Development|ExecuteConsoleCommand "show Splines" 0)
  (Transformation|SetRelativeLocation (Variables|Default|GetIstanbulPin) (CallFunction|LatLontoVector 41.2753 28.7519 254.0) false false)
  (bind _outrownames (DataTable|GetDataTableRowNames "/Game/rotalar.rotalar"))
  (for _array_element _outrownames
    (bind _returnvalue (Utilities|GetDataTableRow "/Game/rotalar.rotalar" _array_element)
      (:then
        (if (== (.sira (Utilities|Struct|BreakFRoutePoint _returnvalue)) 0)
          (bind _returnvalue_2 (AddComponent|AddSplineComponent false))
          (Class|SplineComponent|SetDrawDebug _returnvalue_2 true)
          (Class|SplineComponent|SetUnselectedSplineSegmentColor _returnvalue_2 (Utilities|Struct|MakeLinearColor 0.0 1.0 2.0 1.0))
          (bind _output_get (Variables|Default|SetCurrentSpline _returnvalue_2))
          (Spline|ClearSplinePoints _output_get true))
        (Spline|AddSplinePoint (Variables|Default|GetCurrentSpline) (CallFunction|LatLontoVector (.enlem (Utilities|Struct|BreakFRoutePoint _returnvalue)) (.boylam (Utilities|Struct|BreakFRoutePoint _returnvalue)) 252.0) "Local" true)))))

(event Collision|EventActorBeginOverlap
  (params (OtherActor :type Actor%20Object%20Reference)))

(event EventTick
  (params (DeltaSeconds :type Float%20%28single-precision%29)))

(fn ConstructionScript
  (Transformation|SetRelativeLocation (Variables|Default|GetIstanbulPin) (CallFunction|LatLontoVector 41.2753 28.7519 254.0) false false)
  (bind _outrownames (DataTable|GetDataTableRowNames "/Game/rotalar.rotalar"))
  (for _array_element _outrownames
    (bind _returnvalue (Utilities|GetDataTableRow "/Game/rotalar.rotalar" _array_element)
      (:then
        (if (== (.sira (Utilities|Struct|BreakFRoutePoint _returnvalue)) 0)
          (bind _returnvalue_2 (AddComponent|AddSplineComponent false))
          (Class|SplineComponent|SetDrawDebug _returnvalue_2 true)
          (bind _output_get (Variables|Default|SetCurrentSpline _returnvalue_2))
          (Spline|ClearSplinePoints _output_get true))
        (Spline|AddSplinePoint (Variables|Default|GetCurrentSpline) (CallFunction|LatLontoVector (.enlem (Utilities|Struct|BreakFRoutePoint _returnvalue)) (.boylam (Utilities|Struct|BreakFRoutePoint _returnvalue)) 252.0) "Local" true)))))

(fn LatLontoVector
  (params (Latitude :type Float%20%28double-precision%29) (Longitude :type Float%20%28double-precision%29) (Radius :type Float%20%28double-precision%29))
  (bind _returnvalue (Math|Trig|Cos(Degrees) Latitude))
  (return (Math|Vector|MakeVector (* Radius _returnvalue (Math|Trig|Cos(Degrees) Longitude)) (* Radius _returnvalue (Math|Trig|Sin(Degrees) Longitude)) (* Radius (Math|Trig|Sin(Degrees) Latitude)))))